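; Combat manager for turn-based combat that sets up a fixed three-versus-three battle on BeginPlay.
; It spawns three BP_LeadingRole and three BP_Rebels actors at the world origin and groups each set into a combat team.
; It passes both teams to InitiallizeCombat, which is defined outside these graphs, with the LeadingRole team as the player's.
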(event EventBeginPlay
  (bind _returnvalue (Math|Transform|MakeTransform "0, 0, 0"))
  (Utilities|FlowControl|Sequence
    (:then_0
      (bind _returnvalue_2 (Game|SpawnActorfromClass "/Game/GUAO_TBS/Blueprints/Combat/BP_LeadingRole.BP_LeadingRole_C" _returnvalue "AlwaysSpawn" 0 0))
      (bind _returnvalue_3 (Game|SpawnActorfromClass "/Game/GUAO_TBS/Blueprints/Combat/BP_LeadingRole.BP_LeadingRole_C" _returnvalue "AlwaysSpawn" 0 0))
      (bind _returnvalue_4 (Game|SpawnActorfromClass "/Game/GUAO_TBS/Blueprints/Combat/BP_LeadingRole.BP_LeadingRole_C" _returnvalue "AlwaysSpawn" 0 0)))
    (:then_1
      (bind _returnvalue_5 (Game|SpawnActorfromClass "/Game/GUAO_TBS/Blueprints/Combat/BP_Rebels.BP_Rebels_C" _returnvalue "AlwaysSpawn" 0 0))
      (bind _returnvalue_6 (Game|SpawnActorfromClass "/Game/GUAO_TBS/Blueprints/Combat/BP_Rebels.BP_Rebels_C" _returnvalue "AlwaysSpawn" 0 0))
      (bind _returnvalue_7 (Game|SpawnActorfromClass "/Game/GUAO_TBS/Blueprints/Combat/BP_Rebels.BP_Rebels_C" _returnvalue "AlwaysSpawn" 0 0)))
    (:then_2
      (Class|CombatManager|InitiallizeCombat (Utilities|Array|MakeArray (Utilities|Struct|MakeCombatTeam (Utilities|Array|MakeArray _returnvalue_2 _returnvalue_3 _returnvalue_4)) (Utilities|Struct|MakeCombatTeam (Utilities|Array|MakeArray _returnvalue_5 _returnvalue_6 _returnvalue_7)))))))

(fn ConstructionScript)